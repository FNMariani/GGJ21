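; BP_Patroller is an enemy pawn whose behavior comes from the BT_Patroller behavior tree.
; On BeginPlay it casts its controller to BP_EnemyAIController and runs that tree.
; An unreached AIMoveTo chain remains in the event graph; it would chase the player and, on success, create the lose widget, hide the player mesh and disable the player's collision.
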(event `self.ReceiveTick`
  (params (DeltaSeconds :type "Float (single-precision)")))

(event `self.ReceiveBeginPlay`
  (bind _asbp_enemy_aicontroller (cast `/Game/Blueprints/BP_EnemyAIController` (`self.GetController`)))
  (`AIController.RunBehaviorTree` _asbp_enemy_aicontroller "/Game/AI/BT_Patroller.BT_Patroller"))

(fn `UserConstructionScript`)